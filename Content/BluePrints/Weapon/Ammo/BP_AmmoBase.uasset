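; Base ammo pickup that refills one of four weapon types (Gun, Machine Gun, Shot Gun, Gutlin) when the player walks into its sphere.
; The construction script sets the billboard sprite from the Weapon type.
; On overlap, it adds that type's clamped amount to the Core's ammo count and signals the supplied ammo widget if that weapon is equipped.
; It then refreshes every BP_WeaponBase ammo message, plays a sound and destroys itself.
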(event OnComponentBeginOverlap(Sphere)
  (params (OverlappedComponent :type Primitive%20Component%20Object%20Reference) (OtherActor :type Actor%20Object%20Reference) (OtherComp :type Primitive%20Component%20Object%20Reference) (OtherBodyIndex :type Integer) (bFromSweep :type Boolean) (SweepResult :type Hit%20Result%20Structure%20%28by%20ref%29))
  (if (== OtherActor (Game|GetPlayerCharacter 0))
    (Utilities|FlowControl|Sequence
      (:then_0
        (|AddAmmo))
      (:then_1
        (if (Utilities|Enum|Equal(Enum) (Variables|Default|GetWeapon) (Variables|/Game/BluePrints/GI_Core.GI_Core_C|GetCurrentWeapon (CallFunction|GetCore)))
          (switch Utilities|FlowControl|Switch|SwitchonEnum_Weapon (Variables|Default|GetWeapon)
            (:NewEnumerator0
              (Class|BPIWBAmmo|AddAmmoSignal(Message) (Variables|Default|GetAmmo%20Widget) (Variables|/Game/BluePrints/GI_Core.GI_Core_C|GetCurrentGunAmmo (CallFunction|GetCore))))
            (:NewEnumerator1
              (Class|BPIWBAmmo|AddAmmoSignal(Message) (Variables|Default|GetAmmo%20Widget) (Variables|/Game/BluePrints/GI_Core.GI_Core_C|GetCurrentMachineGunAmmo (CallFunction|GetCore))))
            (:NewEnumerator2
              (Class|BPIWBAmmo|AddAmmoSignal(Message) (Variables|Default|GetAmmo%20Widget) (Variables|/Game/BluePrints/GI_Core.GI_Core_C|GetCurrentShotGunAmmo (CallFunction|GetCore))))
            (:NewEnumerator3
              (Class|BPIWBAmmo|AddAmmoSignal(Message) (Variables|Default|GetAmmo%20Widget) (Variables|/Game/BluePrints/GI_Core.GI_Core_C|GetCurrentGutlinAmmo (CallFunction|GetCore)))))))
      (:then_2
        (bind _outactors (Actor|GetAllActorsOfClass "/Game/BluePrints/Weapon/BP_WeaponBase.BP_WeaponBase_C"))
        (for _array_element _outactors
          (Class|BPIWeaponUse|UpdateAmmo(Message) _array_element)))
      (:then_3
        (Audio|PlaySound2D "/Game/Sounds/TakeAmmo_Cue.TakeAmmo_Cue" 1.0 1.0 0.0 0 0)
        (Actor|DestroyActor)))))

(event EventBeginPlay)

(event Collision|EventActorBeginOverlap
  (params (OtherActor :type Actor%20Object%20Reference)))

(event EventTick
  (params (DeltaSeconds :type Float%20%28single-precision%29)))

(event EventGetAmmoWidget
  (params (AmmoWidget :type WB%20Ammo%20Object%20Reference))
  (Variables|Default|SetAmmo%20Widget AmmoWidget))

(fn ConstructionScript
  (Utilities|FlowControl|Sequence
    (:then_0
      (switch Utilities|FlowControl|Switch|SwitchonEnum_Weapon (Variables|Default|GetWeapon)
        (:NewEnumerator0
          (Variables|Default|SetSprite "/Game/Textures/Kits/ammo-pistol-alt_32px.ammo-pistol-alt_32px"))
        (:NewEnumerator1
          (Variables|Default|SetSprite "/Game/Textures/Kits/ammo-rifle_32px.ammo-rifle_32px"))
        (:NewEnumerator2
          (Variables|Default|SetSprite "/Game/Textures/Kits/ammo-shotgun_32px.ammo-shotgun_32px"))
        (:NewEnumerator3
          (Variables|Default|SetSprite "/Game/Textures/Kits/ammo-rifle-alt_32px.ammo-rifle-alt_32px"))))
    (:then_1
      (Rendering|Components|Sprite|SetSprite (Variables|Default|GetBillboard) (Variables|Default|GetSprite)))))