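; Base weapon Blueprint for the player's hitscan guns, animated with flipbooks and covering gun, machine gun, shotgun and Gutlin types.
; Shoot signals fire once or start a looping cooldown timer for automatics, driving sound, camera animation and a light flash.
; WeaponShoot casts randomly spread camera traces per bullet, with debug drawing, applying damage and spending ammo.
; Per-type ammo persists in the shared Core object, while interface messages update the ammo widget.
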(event Custom|Shoot
  (bind _cooldown (Variables|WeaponSet|GetCoolDown))
  ;[1 0 0.2109] Shoot
  (if (>= (Variables|WeaponSet|GetCurrentAmmo) (Variables|WeaponSet|GetBulletByShot))
    (if (> (Variables|WeaponSet|GetCurrentAmmo) 0)
      (Variables|WeaponSet|SetCanShoot false)
      (Utilities|FlowControl|Sequence
        (:then_0
          (switch Utilities|FlowControl|Switch|SwitchonEnum_WeaponType (Variables|WeaponSet|GetType)
            (:NewEnumerator0
              (Class|BPIWBAmmo|ShootSignal(Message) (Variables|Default|GetAmmo%20Widget) (Variables|WeaponSet|GetCurrentAmmo) (Variables|WeaponSet|GetCoolDown))
              (CallFunction|WeaponShoot)
              (if (Variables|WeaponSet|GetAuto)
                (Utilities|FlowControl|RetriggerableDelay (+ _cooldown 0.1))
                (else
                  (Utilities|FlowControl|Delay _cooldown)))
              (Variables|WeaponSet|SetCanShoot true)
              (Audio|PlaySound2D (Variables|Config|GetEndShootSound) 1.0 1.0 0.0 0 0))))
        (:then_1
          (Sprite|SetFlipbook (Variables|Default|GetFB_Shotgun) (Variables|Config|GetWeaponFlipBookShoot))
          (Audio|PlaySoundatLocation (Variables|Config|GetShootSound) (Transformation|GetActorLocation) "0, 0, 0" 1.0 1.0 0.0 0 0 0 0)
          (Class|BPIWeaponUse|CameraAnimPlaySignalPlayer(Message) (Game|GetPlayerCharacter 0))
          (if (not (Variables|WeaponSet|GetAuto))
            (CallFunction|AnimationEmergencyStop)))
        (:then_2
          (bind _alpha (Timeline|FireLight PlayFromStart)
            (:Update
              (Rendering|Components|Light|SetIntensity (Variables|Default|GetPointLight) (* _alpha (Variables|Config|GetLightIntesivity)))))))
      (else
        (CallFunction|AnimationEmergencyStop)
        (Class|BPIWBAmmo|NotEnoughAmmoSignal(Message) (Variables|Default|GetAmmo%20Widget) :!label _label)))
    (else
      (goto _label))))

(event Custom|AnimationEmergencyStop
  ;[1 0.8203 0] StopShooting
  (Utilities|Time|PauseTimerbyHandle (Variables|Default|GetRifleFireTimer))
  (Utilities|FlowControl|Delay (Class|PaperFlipbookComponent|GetFlipbookLength (Variables|Default|GetFB_Shotgun)))
  (Sprite|SetFlipbook (Variables|Default|GetFB_Shotgun) (Variables|Config|GetWeapon%20Flip%20Book%20Idle)))

(event EventSwitchSignal
  (params (AmmoWidget :type WB%20Ammo%20Object%20Reference))
  (bind _asgi_core (CallFunction|GetCore))
  (bind _asgi_core_2 (CallFunction|GetCore))
  ;[0.4297 1 0] Switch
  (Variables|Default|SetAmmo%20Widget AmmoWidget)
  (Sprite|SetFlipbook (Variables|Default|GetFB_Shotgun) (Variables|Config|GetWeapon%20Flip%20Book%20Idle))
  (Audio|PlaySoundatLocation (Variables|Config|GetSwitchSound) (Transformation|GetActorLocation) "0, 0, 0" 1.0 1.0 0.0 0 0 0 0)
  (Class|BPIWeaponUse|CameraAnimSignalPlayer(Message) (Game|GetPlayerCharacter 0) (Variables|Config|GetCameraAnimation))
  (Rendering|Components|Light|SetLightColor (Variables|Default|GetPointLight) (Variables|Config|GetLightColor) true)
  (Rendering|Lighting|SetAttenuationRadius (Variables|Default|GetPointLight) (Variables|Config|GetLightRange))
  (Utilities|FlowControl|Sequence
    (:then_0
      (switch Utilities|FlowControl|Switch|SwitchonEnum_Weapon (Variables|Config|GetThisWeapon)
        (:NewEnumerator0
          (Variables|WeaponSet|SetCurrentAmmo (Variables|/Game/BluePrints/GI_Core.GI_Core_C|GetCurrentGunAmmo _asgi_core))
          (Variables|WeaponSet|SetAmmoLimit (Variables|/Game/BluePrints/GI_Core.GI_Core_C|GetGunAmmoLimit _asgi_core_2)))
        (:NewEnumerator1
          (Variables|WeaponSet|SetCurrentAmmo (Variables|/Game/BluePrints/GI_Core.GI_Core_C|GetCurrentMachineGunAmmo _asgi_core))
          (Variables|WeaponSet|SetAmmoLimit (Variables|/Game/BluePrints/GI_Core.GI_Core_C|GetMachineGunAmmoLimit _asgi_core_2)))
        (:NewEnumerator2
          (Variables|WeaponSet|SetCurrentAmmo (Variables|/Game/BluePrints/GI_Core.GI_Core_C|GetCurrentShotGunAmmo _asgi_core))
          (Variables|WeaponSet|SetAmmoLimit (Variables|/Game/BluePrints/GI_Core.GI_Core_C|GetShotGunAmmoLimit _asgi_core_2)))
        (:NewEnumerator3
          (Variables|WeaponSet|SetCurrentAmmo (Variables|/Game/BluePrints/GI_Core.GI_Core_C|GetCurrentGutlinAmmo _asgi_core))
          (Variables|WeaponSet|SetAmmoLimit (Variables|/Game/BluePrints/GI_Core.GI_Core_C|GetGutlinAmmoLimit _asgi_core_2)))))
    (:then_1
      (Class|BPIWBAmmo|SwitchSignal(Message) (Variables|Default|GetAmmo%20Widget) (Variables|WeaponSet|GetCurrentAmmo) (Variables|WeaponSet|GetAmmoLimit) (Variables|Config|GetName)))))

(event EventUpdateAmmo
  ;[1 0 0.2109] Shoot
  (CallFunction|NewAmmo))

(event EventShootSignal
  (bind _cooldown (Variables|WeaponSet|GetCoolDown))
  ;[1 0 0.2109] Shoot
  (if (Variables|WeaponSet|GetCanShoot)
    (if (Variables|WeaponSet|GetAuto)
      (bind _returnvalue (Utilities|Time|SetTimerbyEvent (delegate Custom|Shoot) (Variables|WeaponSet|GetCoolDown) true))
      (Variables|Default|SetRifleFireTimer _returnvalue))
    (if (>= (Variables|WeaponSet|GetCurrentAmmo) (Variables|WeaponSet|GetBulletByShot))
      (if (> (Variables|WeaponSet|GetCurrentAmmo) 0)
        (Variables|WeaponSet|SetCanShoot false)
        (Utilities|FlowControl|Sequence
          (:then_0
            (switch Utilities|FlowControl|Switch|SwitchonEnum_WeaponType (Variables|WeaponSet|GetType)
              (:NewEnumerator0
                (Class|BPIWBAmmo|ShootSignal(Message) (Variables|Default|GetAmmo%20Widget) (Variables|WeaponSet|GetCurrentAmmo) (Variables|WeaponSet|GetCoolDown))
                (CallFunction|WeaponShoot)
                (if (Variables|WeaponSet|GetAuto)
                  (Utilities|FlowControl|RetriggerableDelay (+ _cooldown 0.1))
                  (else
                    (Utilities|FlowControl|Delay _cooldown)))
                (Variables|WeaponSet|SetCanShoot true)
                (Audio|PlaySound2D (Variables|Config|GetEndShootSound) 1.0 1.0 0.0 0 0))))
          (:then_1
            (Sprite|SetFlipbook (Variables|Default|GetFB_Shotgun) (Variables|Config|GetWeaponFlipBookShoot))
            (Audio|PlaySoundatLocation (Variables|Config|GetShootSound) (Transformation|GetActorLocation) "0, 0, 0" 1.0 1.0 0.0 0 0 0 0)
            (Class|BPIWeaponUse|CameraAnimPlaySignalPlayer(Message) (Game|GetPlayerCharacter 0))
            (if (not (Variables|WeaponSet|GetAuto))
              (CallFunction|AnimationEmergencyStop)))
          (:then_2
            (bind _alpha (Timeline|FireLight PlayFromStart)
              (:Update
                (Rendering|Components|Light|SetIntensity (Variables|Default|GetPointLight) (* _alpha (Variables|Config|GetLightIntesivity)))))))
        (else
          (CallFunction|AnimationEmergencyStop)
          (Class|BPIWBAmmo|NotEnoughAmmoSignal(Message) (Variables|Default|GetAmmo%20Widget) :!label _label)))
      (else
        (goto _label)))))

(event EventStopShootSignal
  ;[1 0.8203 0] StopShooting
  (if (Variables|WeaponSet|GetAuto)
    (Utilities|Time|PauseTimerbyHandle (Variables|Default|GetRifleFireTimer))
    (Utilities|FlowControl|Delay (Class|PaperFlipbookComponent|GetFlipbookLength (Variables|Default|GetFB_Shotgun)) :!label _label)
    (elif (not (Variables|WeaponSet|GetCanShoot))
      (goto _label)
      (else
        _)))
  (Sprite|SetFlipbook (Variables|Default|GetFB_Shotgun) (Variables|Config|GetWeapon%20Flip%20Book%20Idle)))

(fn ConstructionScript)

(fn WeaponShoot
  (bind (_returnvalue _returnvalue2) (|LineTraceAndSpread))
  (bind (_returnvalue_2 _returnvalue2_2 _returnvalue3) (|DecalSizeGenerator))
  (bind _linetracecolor (Variables|Debug|GetLineTraceColor))
  (if (>= (Variables|WeaponSet|GetCurrentAmmo) (Variables|WeaponSet|GetBulletByShot))
    (for _index (range 0 (- (Variables|WeaponSet|GetBulletByShot) 1))
      (bind _outhit (Collision|LineTraceByChannel _returnvalue _returnvalue2 "TraceTypeQuery1" false 0 "ForDuration" true _linetracecolor _linetracecolor))
      (bind _result (Math|Integer|DecrementInt (Variables|WeaponSet|GetCurrentAmmo))
        (:%20%20
          (Variables|WeaponSet|SetCurrentAmmo _result)
          (Utilities|FlowControl|Sequence
            (:then_0
              (if (.bBlockingHit (Collision|BreakHitResult _outhit))
                (Game|Damage|ApplyDamage (.HitActor (Collision|BreakHitResult _outhit)) (Variables|WeaponSet|GetDamage) (Game|GetPlayerController 0) self)
                (if (== (Utilities|GetClass (.HitActor (Collision|BreakHitResult _outhit))) "/Game/BluePrints/Enemy/BP_Doll.BP_Doll_C")
                  (Variables|Default|SetParticle 0)
                  (else
                    (Variables|Default|SetParticle 0)))
                (Effects|SpawnEmitteratLocation (Variables|Default|GetParticle) (.Location (Collision|BreakHitResult _outhit)) (Math|Conversions|RotationFromXVector (.ImpactNormal (Collision|BreakHitResult _outhit))) (Math|Vector|MakeVector _returnvalue_2 _returnvalue2_2 _returnvalue3))))
            (:then_1
              (|SaveCurrentAmmoValue_GI))))))
    (else
      (for _index_2 (range 0 (Utilities|Operators|Subtract (Variables|WeaponSet|GetBulletByShot) (Variables|WeaponSet|GetCurrentAmmo)))
        (bind _outhit_2 (Collision|LineTraceByChannel _returnvalue _returnvalue2 "TraceTypeQuery1" false 0 "ForDuration" true _linetracecolor _linetracecolor))
        (bind _result_2 (Math|Integer|DecrementInt (Variables|WeaponSet|GetCurrentAmmo))
          (:%20%20
            (Variables|WeaponSet|SetCurrentAmmo _result_2)
            (Utilities|FlowControl|Sequence
              (:then_0
                (if (.bBlockingHit (Collision|BreakHitResult _outhit_2))
                  (Game|Damage|ApplyDamage (.HitActor (Collision|BreakHitResult _outhit_2)) (Variables|WeaponSet|GetDamage) (Game|GetPlayerController 0) self)
                  (if (== (Utilities|GetClass (.HitActor (Collision|BreakHitResult _outhit_2))) "/Game/BluePrints/Enemy/BP_Doll.BP_Doll_C")
                    (Variables|Default|SetParticle 0)
                    (else
                      (Variables|Default|SetParticle 0)))
                  (Effects|SpawnEmitteratLocation (Variables|Default|GetParticle) (.Location (Collision|BreakHitResult _outhit_2)) (Math|Conversions|RotationFromXVector (.ImpactNormal (Collision|BreakHitResult _outhit_2))) (Math|Vector|MakeVector _returnvalue_2 _returnvalue2_2 _returnvalue3))))
              (:then_1
                (|SaveCurrentAmmoValue_GI))))))))
  (Utilities|FlowControl|Sequence
    (:then_1
      (return true))))

(fn NewAmmo
  (switch Utilities|FlowControl|Switch|SwitchonEnum_Weapon (Variables|Config|GetThisWeapon)
    (:NewEnumerator0
      (Variables|WeaponSet|SetCurrentAmmo (Variables|/Game/BluePrints/GI_Core.GI_Core_C|GetCurrentGunAmmo (CallFunction|GetCore))))
    (:NewEnumerator1
      (Variables|WeaponSet|SetCurrentAmmo (Variables|/Game/BluePrints/GI_Core.GI_Core_C|GetCurrentMachineGunAmmo (CallFunction|GetCore))))
    (:NewEnumerator2
      (Variables|WeaponSet|SetCurrentAmmo (Variables|/Game/BluePrints/GI_Core.GI_Core_C|GetCurrentShotGunAmmo (CallFunction|GetCore))))
    (:NewEnumerator3
      (Variables|WeaponSet|SetCurrentAmmo (Variables|/Game/BluePrints/GI_Core.GI_Core_C|GetCurrentGutlinAmmo (CallFunction|GetCore))))))

(fn GetAmmoFull
  (return (and (== (Variables|WeaponSet|GetCurrentAmmo) (Variables|WeaponSet|GetAmmoLimit)) (!= (Variables|WeaponSet|GetAmmoLimit) -1))))