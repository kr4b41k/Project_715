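; Ability entity for a falling-star magic attack that drops from its spawn point and explodes on impact.
; A timeline drives downward sphere traces with growing radius and step, advancing a stored location without moving the actor and ignoring BP_Doll actors.
; Each miss applies lighter radial magic damage with a flare.
; A hit stops the timeline, re-traces, then deals heavy damage with explosion emitters, sparing the player.
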(event Custom|Stop
  (bind _alpha (Timeline|StarFall Stop)
    (:Update
      (Utilities|FlowControl|Delay 0.02)
      (bind _outactors (Actor|GetAllActorsOfClass "/Game/BluePrints/Enemy/BP_Doll.BP_Doll_C"))
      (Variables|Default|SetRadius (* _alpha 5e+02))
      (bind (_outhit _returnvalue) (Collision|SphereTraceByChannel (Variables|Default|GetActorLocation) (Math|Vector|MakeVector (.x (Variables|Default|GetActorLocation)) (.y (Variables|Default|GetActorLocation)) (- (.z (Variables|Default|GetActorLocation)) (* _alpha (Variables|Default|GetFallDelta)))) (Variables|Default|GetRadius) "TraceTypeQuery1" false _outactors "None"))
      (if _returnvalue
        (Variables|Default|SetActorLocation (.Location (Collision|BreakHitResult _outhit)))
        (bind (_outhit_2 _returnvalue_2) (Collision|SphereTraceByChannel (Variables|Default|GetActorLocation) (Math|Vector|MakeVector (.x (Variables|Default|GetActorLocation)) (.y (Variables|Default|GetActorLocation)) (- (.z (Variables|Default|GetActorLocation)) (Variables|Default|GetRadius))) (Variables|Default|GetRadius) "TraceTypeQuery1" false 0 "ForDuration"))
        (if _returnvalue_2
          (Variables|Default|SetActorLocation (.Location (Collision|BreakHitResult _outhit_2)))
          (else
            (Variables|Default|SetActorLocation (.TraceEnd (Collision|BreakHitResult _outhit_2)))))
        (CallFunction|Stop)
        (Class|GameplayStatics|ApplyRadialDamagewithFalloff 4e+02 1.5e+02 (Variables|Default|GetActorLocation) 2.5e+02 6e+02 5.0 "/Game/BluePrints/VitalityMana/DMT_Magic.DMT_Magic_C" (Utilities|Array|MakeArray (Game|GetPlayerCharacter 0)) (.HitActor (Collision|BreakHitResult _outhit_2)) (Game|GetPlayerController 0) "ECC_Visibility")
        (Effects|SpawnEmitteratLocation "/Game/Assets/InfinityBladeEffects/Effects/FX_Cines/cinema03/P_CIN_IB_Explosion_Flare.P_CIN_IB_Explosion_Flare" (Variables|Default|GetActorLocation) "0, 0, 0" "2.000000,2.000000,2.000000")
        (Variables|Default|SetActorLocation (Math|Vector|MakeVector (.x (Variables|Default|GetActorLocation)) (.y (Variables|Default|GetActorLocation)) (- (.z (Variables|Default|GetActorLocation)) (Variables|Default|GetRadius))))
        (Effects|SpawnEmitteratLocation "/Game/UsedAssets/P_CIN_IB_Explosion.P_CIN_IB_Explosion" (Variables|Default|GetActorLocation))
        (Effects|SpawnEmitteratLocation "/Game/UsedAssets/P_CIN_IB_Explosion_02.P_CIN_IB_Explosion_02" (Variables|Default|GetActorLocation) "0, 0, 0" "10.000000,10.000000,10.000000")
        (else
          (Variables|Default|SetActorLocation (.TraceEnd (Collision|BreakHitResult _outhit)))
          (Class|GameplayStatics|ApplyRadialDamagewithFalloff 1e+02 3e+01 (Variables|Default|GetActorLocation) 1e+02 3e+02 5.0 "/Game/BluePrints/VitalityMana/DMT_Magic.DMT_Magic_C" (Utilities|Array|MakeArray (Game|GetPlayerCharacter 0)) (.HitActor (Collision|BreakHitResult _outhit)) (Game|GetPlayerController 0) "ECC_Visibility")
          (Effects|SpawnEmitteratLocation "/Game/UsedAssets/P_CIN_IB_Explosion_Flare.P_CIN_IB_Explosion_Flare" (Variables|Default|GetActorLocation) "0, 0, 0" "2.000000,2.000000,2.000000"))))))

(event EventBeginPlay
  (|CallParentFunction)
  (Variables|Default|SetActorLocation (Transformation|GetActorLocation))
  (bind _alpha (Timeline|StarFall Play)
    (:Update
      (Utilities|FlowControl|Delay 0.02)
      (bind _outactors (Actor|GetAllActorsOfClass "/Game/BluePrints/Enemy/BP_Doll.BP_Doll_C"))
      (Variables|Default|SetRadius (* _alpha 5e+02))
      (bind (_outhit _returnvalue) (Collision|SphereTraceByChannel (Variables|Default|GetActorLocation) (Math|Vector|MakeVector (.x (Variables|Default|GetActorLocation)) (.y (Variables|Default|GetActorLocation)) (- (.z (Variables|Default|GetActorLocation)) (* _alpha (Variables|Default|GetFallDelta)))) (Variables|Default|GetRadius) "TraceTypeQuery1" false _outactors "None"))
      (if _returnvalue
        (Variables|Default|SetActorLocation (.Location (Collision|BreakHitResult _outhit)))
        (bind (_outhit_2 _returnvalue_2) (Collision|SphereTraceByChannel (Variables|Default|GetActorLocation) (Math|Vector|MakeVector (.x (Variables|Default|GetActorLocation)) (.y (Variables|Default|GetActorLocation)) (- (.z (Variables|Default|GetActorLocation)) (Variables|Default|GetRadius))) (Variables|Default|GetRadius) "TraceTypeQuery1" false 0 "ForDuration"))
        (if _returnvalue_2
          (Variables|Default|SetActorLocation (.Location (Collision|BreakHitResult _outhit_2)))
          (else
            (Variables|Default|SetActorLocation (.TraceEnd (Collision|BreakHitResult _outhit_2)))))
        (CallFunction|Stop)
        (Class|GameplayStatics|ApplyRadialDamagewithFalloff 4e+02 1.5e+02 (Variables|Default|GetActorLocation) 2.5e+02 6e+02 5.0 "/Game/BluePrints/VitalityMana/DMT_Magic.DMT_Magic_C" (Utilities|Array|MakeArray (Game|GetPlayerCharacter 0)) (.HitActor (Collision|BreakHitResult _outhit_2)) (Game|GetPlayerController 0) "ECC_Visibility")
        (Effects|SpawnEmitteratLocation "/Game/Assets/InfinityBladeEffects/Effects/FX_Cines/cinema03/P_CIN_IB_Explosion_Flare.P_CIN_IB_Explosion_Flare" (Variables|Default|GetActorLocation) "0, 0, 0" "2.000000,2.000000,2.000000")
        (Variables|Default|SetActorLocation (Math|Vector|MakeVector (.x (Variables|Default|GetActorLocation)) (.y (Variables|Default|GetActorLocation)) (- (.z (Variables|Default|GetActorLocation)) (Variables|Default|GetRadius))))
        (Effects|SpawnEmitteratLocation "/Game/UsedAssets/P_CIN_IB_Explosion.P_CIN_IB_Explosion" (Variables|Default|GetActorLocation))
        (Effects|SpawnEmitteratLocation "/Game/UsedAssets/P_CIN_IB_Explosion_02.P_CIN_IB_Explosion_02" (Variables|Default|GetActorLocation) "0, 0, 0" "10.000000,10.000000,10.000000")
        (else
          (Variables|Default|SetActorLocation (.TraceEnd (Collision|BreakHitResult _outhit)))
          (Class|GameplayStatics|ApplyRadialDamagewithFalloff 1e+02 3e+01 (Variables|Default|GetActorLocation) 1e+02 3e+02 5.0 "/Game/BluePrints/VitalityMana/DMT_Magic.DMT_Magic_C" (Utilities|Array|MakeArray (Game|GetPlayerCharacter 0)) (.HitActor (Collision|BreakHitResult _outhit)) (Game|GetPlayerController 0) "ECC_Visibility")
          (Effects|SpawnEmitteratLocation "/Game/UsedAssets/P_CIN_IB_Explosion_Flare.P_CIN_IB_Explosion_Flare" (Variables|Default|GetActorLocation) "0, 0, 0" "2.000000,2.000000,2.000000"))))))

(event Collision|EventActorBeginOverlap
  (params (OtherActor :type Actor%20Object%20Reference))
  (|CallParentFunction OtherActor) ; This node is disabled and will not be called.\nDrag off pins to build functionality.
)

(event EventTick
  (params (DeltaSeconds :type Float%20%28single-precision%29))
  (|CallParentFunction DeltaSeconds) ; This node is disabled and will not be called.\nDrag off pins to build functionality.
)

(fn ConstructionScript
  (|CallParentFunction))