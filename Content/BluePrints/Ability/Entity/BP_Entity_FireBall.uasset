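; Fireball projectile entity that explodes on impact, dealing radial magic damage while sparing player character 0.
; The projectile movement's bounce event serves as the hit trigger, filtering out hits on that player.
; A valid hit spawns spark and asphalt particles angled between impact velocity and surface normal, applies damage with the hit actor as causer, then destroys the fireball.
; BeginPlay also destroys it after a fixed lifetime.
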(event OnProjectileBounce(ProjectileMovement)
  (params (ImpactResult :type Hit%20Result%20Structure%20%28by%20ref%29) (ImpactVelocity :type Vector%20%28by%20ref%29 :default "0, 0, 0"))
  (bind (_bblockinghit _binitialoverlap _time _distance _location _impactpoint _normal _impactnormal _physmat _hitactor) (Collision|BreakHitResult ImpactResult))
  (bind _returnvalue (Class|KismetMathLibrary|VectorSlerpVectortoDirection ImpactVelocity _impactnormal 0.9))
  (bind _returnvalue_2 (Math|Conversions|RotationFromXVector _returnvalue))
  (Variables|Default|SetOther%20Actor _hitactor)
  (Variables|Default|SetLocation _location)
  (if _bblockinghit
    (if (or (!= (Game|GetPlayerCharacter 0) (Variables|Default|GetOther%20Actor)) (== (Variables|Default|GetOther%20Actor) self))
      (Effects|SpawnEmitteratLocation "/Game/UsedAssets/P_Sparks_G.P_Sparks_G" (Variables|Default|GetLocation) _returnvalue_2 (Math|Vector|MakeVector 0.8 0.8 0.8))
      (Effects|SpawnEmitteratLocation "/Game/UsedAssets/P_Asphalt.P_Asphalt" (Variables|Default|GetLocation) _returnvalue_2 (Math|Vector|MakeVector 0.8 0.8 0.8))
      (Game|Damage|ApplyRadialDamage 5e+01 (Variables|Default|GetLocation) 1.5e+02 "/Game/BluePrints/VitalityMana/DMT_Magic.DMT_Magic_C" (Utilities|Array|MakeArray (Game|GetPlayerCharacter 0)) (Variables|Default|GetOther%20Actor) (Game|GetPlayerController 0) false "ECC_Visibility")
      (Actor|DestroyActor))))

(event EventBeginPlay
  (Utilities|FlowControl|Delay 15.0)
  (Actor|DestroyActor))

(fn ConstructionScript)