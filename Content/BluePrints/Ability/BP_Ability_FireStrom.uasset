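; Fire storm ability actor that, on AbilitySignal, sprays damaging fire along the player camera's view.
; Each volley fires several capsule traces toward randomly spread points at range, spawning two impact emitters and applying damage on blocking hits.
; A Delay inside the loop feeds back into the volley to repeat it, with a whoosh sound after each pass.
; GetTimeOfAbilityUse exposes the ability's use time.
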(event EventBeginPlay
  (|CallParentFunction))

(event Collision|EventActorBeginOverlap
  (params (OtherActor :type Actor%20Object%20Reference))
  (|CallParentFunction OtherActor) ; This node is disabled and will not be called.\nDrag off pins to build functionality.
)

(event EventTick
  (params (DeltaSeconds :type Float%20%28single-precision%29))
  (|CallParentFunction DeltaSeconds) ; This node is disabled and will not be called.\nDrag off pins to build functionality.
)

(event EventAbilitySignal
  (bind _returnvalue (Game|GetPlayerCameraManager 0))
  (bind _spread (Variables|Default|GetSpread))
  (bind _spread_2 (Variables|Default|GetSpread))
  (bind _spread_3 (Variables|Default|GetSpread))
  (bind _returnvalue_2 (Transformation|GetActorLocation _returnvalue))
  (for _index (range 0 7) :!label _label
    (bind (_outhit _returnvalue_3) (Collision|CapsuleTraceByChannel _returnvalue_2 (+ (+ _returnvalue_2 (* (Transformation|GetActorForwardVector _returnvalue) (Variables|Default|GetRange))) (Math|Vector|MakeVector (Math|Random|RandomFloatinRange (* _spread_2 -1.0) _spread_2) (Math|Random|RandomFloatinRange (* _spread_3 -1.0) _spread_3) (Math|Random|RandomFloatinRange (* _spread -1.0) _spread))) 3e+01 3e+01 "TraceTypeQuery1" true 0 "None"))
    (Utilities|FlowControl|Sequence
      (:then_0
        (for _index_2 (range 0 18)
          (Utilities|FlowControl|Delay 0.12)
          (goto _label)))
      (:then_1
        (if _returnvalue_3
          (if (.bBlockingHit (Collision|BreakHitResult _outhit))
            (Effects|SpawnEmitteratLocation 0 (.Location (Collision|BreakHitResult _outhit)) (Math|Conversions|RotationFromXVector (.ImpactNormal (Collision|BreakHitResult _outhit))) (Math|Vector|MakeVector 2.0 2.0 2.0))
            (Effects|SpawnEmitteratLocation 0 (.Location (Collision|BreakHitResult _outhit)) (Math|Conversions|RotationFromXVector (.ImpactNormal (Collision|BreakHitResult _outhit))) (Math|Vector|MakeVector 0.8 0.8 0.8))
            (Game|Damage|ApplyDamage (.HitActor (Collision|BreakHitResult _outhit)) 5.0 (Game|GetPlayerController 0) self "/Game/BluePrints/VitalityMana/DMT_Damage.DMT_Damage_C"))))))
  (Audio|PlaySound2D "/Game/Sounds/mixkit-short-fire-whoosh-1345_Cue.mixkit-short-fire-whoosh-1345_Cue" 0.3 1.3 0.15 0 0))

(fn ConstructionScript
  (|CallParentFunction))

(fn GetTimeOfAbilityUse
  (return (Variables|Default|GetAbilityUseTime)))