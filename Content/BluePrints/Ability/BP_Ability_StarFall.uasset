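; Star Fall ability that, on its signal, spawns an entity high above the point the player camera aims at.
; Three debug-drawn visibility traces, all ignoring BP_Doll actors, chain together: forward from the camera to Range, a short step back toward it, then vertically to a fixed world height.
; Each trace passes on its hit or end point, so obstructions cap the final spawn location.
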(event EventBeginPlay
  (|CallParentFunction) ; This node is disabled and will not be called.\nDrag off pins to build functionality.
)

(event Collision|EventActorBeginOverlap
  (params (OtherActor :type Actor%20Object%20Reference))
  (|CallParentFunction OtherActor) ; This node is disabled and will not be called.\nDrag off pins to build functionality.
)

(event EventTick
  (params (DeltaSeconds :type Float%20%28single-precision%29))
  (|CallParentFunction DeltaSeconds) ; This node is disabled and will not be called.\nDrag off pins to build functionality.
)

(event EventAbilitySignal
  (bind _returnvalue (Game|GetPlayerCameraManager 0))
  (bind _returnvalue_2 (Transformation|GetActorForwardVector _returnvalue))
  (Variables|Default|SetCameraLocation (Camera|GetCameraLocation _returnvalue))
  (Variables|Default|SetActorForwardVector (Math|Vector|MakeVector (.x _returnvalue_2) (.y _returnvalue_2) (.z _returnvalue_2)))
  (bind _outactors (Actor|GetAllActorsOfClass "/Game/BluePrints/Enemy/BP_Doll.BP_Doll_C"))
  (bind (_outhit _returnvalue_3) (Collision|LineTraceByChannel (Variables|Default|GetCameraLocation) (+ (Variables|Default|GetCameraLocation) (* (Variables|Default|GetActorForwardVector) (Variables|Default|GetRange))) "TraceTypeQuery1" false _outactors "ForDuration"))
  (if _returnvalue_3
    (Variables|Default|SetJointBackLocation (.Location (Collision|BreakHitResult _outhit)))
    (else
      (Variables|Default|SetJointBackLocation (.TraceEnd (Collision|BreakHitResult _outhit)))))
  (bind (_outhit_2 _returnvalue_4) (Collision|LineTraceByChannel (Variables|Default|GetJointBackLocation) (+ (Variables|Default|GetJointBackLocation) (* (Variables|Default|GetActorForwardVector) -1.0 2e+02)) "TraceTypeQuery1" false _outactors "ForDuration" true "(R=0.190566,G=0.000000,B=1.000000,A=1.000000)" "(R=1.000000,G=0.589374,B=0.000000,A=1.000000)"))
  (if _returnvalue_4
    (Variables|Default|SetStarSpawnLocation (.Location (Collision|BreakHitResult _outhit_2)))
    (else
      (Variables|Default|SetStarSpawnLocation (.TraceEnd (Collision|BreakHitResult _outhit_2)))))
  (bind (_outhit_3 _returnvalue_5) (Collision|LineTraceByChannel (Variables|Default|GetStarSpawnLocation) (Math|Vector|MakeVector (.x (Variables|Default|GetStarSpawnLocation)) (.y (Variables|Default|GetStarSpawnLocation)) 4e+03) "TraceTypeQuery1" false _outactors "ForDuration" true "(R=0.190566,G=0.000000,B=1.000000,A=1.000000)" "(R=1.000000,G=0.589374,B=0.000000,A=1.000000)"))
  (if _returnvalue_5
    (Variables|Default|SetStarLocation (.Location (Collision|BreakHitResult _outhit_3)))
    (else
      (Variables|Default|SetStarLocation (.TraceEnd (Collision|BreakHitResult _outhit_3)))))
  (CallFunction|SpawnEntity (Math|Transform|MakeTransform (Variables|Default|GetStarLocation) "0, 0, 0" "1.000000,1.000000,1.000000")))

(fn ConstructionScript
  (|CallParentFunction))