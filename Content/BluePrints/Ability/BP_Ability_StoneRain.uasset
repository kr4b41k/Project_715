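; Stone Rain ability actor that spawns its Entity class in the world based on the player's camera aim.
; On AbilitySignal, it line-traces forward from the camera by Range.
; Only when that trace misses, a second trace runs from its hit location backward along the view direction for a third of Range.
; The Entity spawns at the second trace's hit location with the player as instigator, and both traces draw debug lines.
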(event EventBeginPlay
  (|CallParentFunction) ; This node is disabled and will not be called.\nDrag off pins to build functionality.
)

(event Collision|EventActorBeginOverlap
  (params (OtherActor :type Actor%20Object%20Reference))
  (|CallParentFunction OtherActor) ; This node is disabled and will not be called.\nDrag off pins to build functionality.
)

(event EventTick
  (params (DeltaSeconds :type Float%20%28single-precision%29))
  (|CallParentFunction DeltaSeconds) ; This node is disabled and will not be called.\nDrag off pins to build functionality.
)

(event EventAbilitySignal
  (bind _returnvalue (Game|GetPlayerCameraManager 0))
  (Variables|Default|SetCameraLocation (Camera|GetCameraLocation _returnvalue))
  (Variables|Default|SetActorForwardVector (Transformation|GetActorForwardVector _returnvalue))
  (bind (_outhit _returnvalue_2) (Collision|LineTraceByChannel (Variables|Default|GetCameraLocation) (+ (Variables|Default|GetCameraLocation) (* (Variables|Default|GetActorForwardVector) (Variables|Default|GetRange))) "TraceTypeQuery1" false 0 "ForDuration"))
  (if (not _returnvalue_2)
    (bind _outhit_2 (Collision|LineTraceByChannel (.Location (Collision|BreakHitResult _outhit)) (+ (.Location (Collision|BreakHitResult _outhit)) (* (* (Variables|Default|GetActorForwardVector) -1.0) (/ (Variables|Default|GetRange) 3.0))) "TraceTypeQuery1" false 0 "ForDuration"))
    (Game|SpawnActorfromClass (Variables|Default|GetEntity) (Math|Transform|MakeTransform (.Location (Collision|BreakHitResult _outhit_2)) "0, 0, 0" "1.000000,1.000000,1.000000") "AlwaysSpawn" "MultiplyWithRoot" self (Game|GetPlayerCharacter 0))))

(fn ConstructionScript
  (|CallParentFunction))