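; Ability pickup actor that grants the player an ability when touched, shown as a billboard spellbook.
; The construction script maps AbilityType to a book sprite and an Ability class, then applies the sprite to the Billboard.
; Only Fire Storm has its own ability class; every other type is assigned BP_AbilityBase.
; When the player character overlaps the Sphere, it sends the Ability through AbilityPickUpMessage and destroys itself.
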(event OnComponentBeginOverlap(Sphere)
  (params (OverlappedComponent :type Primitive%20Component%20Object%20Reference) (OtherActor :type Actor%20Object%20Reference) (OtherComp :type Primitive%20Component%20Object%20Reference) (OtherBodyIndex :type Integer) (bFromSweep :type Boolean) (SweepResult :type Hit%20Result%20Structure%20%28by%20ref%29))
  (bind _returnvalue (Game|GetPlayerCharacter 0))
  (if (== OtherActor _returnvalue)
    (Class|BPIAbilityPickUp|AbilityPickUp(Message) _returnvalue (Variables|Default|GetAbility))
    (Actor|DestroyActor)))

(event EventBeginPlay)

(event Collision|EventActorBeginOverlap
  (params (OtherActor :type Actor%20Object%20Reference)))

(event EventTick
  (params (DeltaSeconds :type Float%20%28single-precision%29)))

(fn ConstructionScript
  (Utilities|FlowControl|Sequence
    (:then_0
      (switch Utilities|FlowControl|Switch|SwitchonEnum_Ability (Variables|Default|GetAbilityType)
        (:NewEnumerator0
          (Variables|Default|SetSprite "/Game/Textures/Magic/AbilityIcon/FIreStormBook.FIreStormBook")
          (Variables|Default|SetAbility "/Game/BluePrints/Ability/BP_Ability_FireStrom.BP_Ability_FireStrom_C"))
        (:NewEnumerator1
          (Variables|Default|SetSprite "/Game/Textures/Magic/AbilityIcon/StoneRainBook.StoneRainBook")
          (Variables|Default|SetAbility "/Game/BluePrints/Ability/BP_AbilityBase.BP_AbilityBase_C"))
        (:NewEnumerator2
          (Variables|Default|SetSprite "/Game/Textures/Magic/AbilityIcon/StarFallBook.StarFallBook")
          (Variables|Default|SetAbility "/Game/BluePrints/Ability/BP_AbilityBase.BP_AbilityBase_C"))
        (:NewEnumerator3
          (Variables|Default|SetSprite "/Game/Textures/Magic/AbilityIcon/GhostArmyBook.GhostArmyBook")
          (Variables|Default|SetAbility "/Game/BluePrints/Ability/BP_AbilityBase.BP_AbilityBase_C"))
        (:NewEnumerator4
          (Variables|Default|SetSprite "/Game/Textures/Magic/AbilityIcon/PricklyGrassBook.PricklyGrassBook")
          (Variables|Default|SetAbility "/Game/BluePrints/Ability/BP_AbilityBase.BP_AbilityBase_C"))
        (:NewEnumerator5
          (Variables|Default|SetSprite "/Game/Textures/Magic/AbilityIcon/GravityZeroBook.GravityZeroBook")
          (Variables|Default|SetAbility "/Game/BluePrints/Ability/BP_AbilityBase.BP_AbilityBase_C"))
        (:NewEnumerator6
          (Variables|Default|SetSprite "/Game/Textures/Magic/AbilityIcon/StasisBook.StasisBook")
          (Variables|Default|SetAbility "/Game/BluePrints/Ability/BP_AbilityBase.BP_AbilityBase_C"))
        (:NewEnumerator7
          (Variables|Default|SetSprite "/Game/Textures/Magic/AbilityIcon/ThunderBoltBook.ThunderBoltBook")
          (Variables|Default|SetAbility "/Game/BluePrints/Ability/BP_AbilityBase.BP_AbilityBase_C"))
        (:NewEnumerator8
          (Variables|Default|SetSprite "/Game/Textures/Magic/AbilityIcon/DeathCurseBook.DeathCurseBook")
          (Variables|Default|SetAbility "/Game/BluePrints/Ability/BP_AbilityBase.BP_AbilityBase_C"))))
    (:then_1
      (Rendering|Components|Sprite|SetSprite (Variables|Default|GetBillboard) (Variables|Default|GetSprite)))))