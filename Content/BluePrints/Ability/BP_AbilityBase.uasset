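; BP_AbilityBase is a base Blueprint for abilities, holding a sprite, a mana cost and a use time.
; On BeginPlay it applies its Sprite variable to the PaperSprite component.
; Getters expose ManaCost and AbilityUseTime, while a separate GetTimeOfAbilityUse_0 function returns a hardcoded duration instead of the variable.
; It contains no activation or effect logic.
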(event EventBeginPlay
  (Rendering|Components|Sprite|SetSprite (Variables|Default|GetPaperSprite) (Variables|Default|GetSprite)))

(event Collision|EventActorBeginOverlap
  (params (OtherActor :type Actor%20Object%20Reference)))

(event EventTick
  (params (DeltaSeconds :type Float%20%28single-precision%29)))

(fn ConstructionScript)

(fn GetTimeOfAbilityUse0
  (return 3.0))

(fn GetManaCost
  (return (Variables|Default|GetManaCost)))

(fn GetTimeOfAbilityUse
  (return (Variables|Default|GetAbilityUseTime)))