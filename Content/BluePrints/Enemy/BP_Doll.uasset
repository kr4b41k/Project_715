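; BP_Doll is a damageable doll enemy shown as a Doom-style billboard sprite with directional flipbooks.
; On a throttled Tick, the sprite yaws toward the player camera; dot products of actor axes and player direction give angle and side, selecting the idle flipbook while alive.
; The rearmost sector reuses FrontIdle.
; Damage lowers clamped HP with a grunt; at zero it disables capsule collision, plays death effects and flipbook, then destroys itself.
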(event EventBeginPlay)

(event Collision|EventActorBeginOverlap
  (params (OtherActor :type Actor%20Object%20Reference)))

(event EventTick
  (params (DeltaSeconds :type Float%20%28single-precision%29))
  (Utilities|FlowControl|Delay 0.083333)
  (if (Variables|Default|GetDie)
    (Utilities|SpriteFacePlayer
      (:Out
        (Utilities|GetAnemyAngle)))
    (else
      (Utilities|SpriteFacePlayer
        (:Out
          (Utilities|GetAnemyAngle
            (:out
              (Utilities|CalculateFB))))))))

(event Game|Damage|EventAnyDamage
  (params (Damage :type Float%20%28single-precision%29) (DamageType :type Damage%20Type%20Object%20Reference) (InstigatedBy :type Controller%20Object%20Reference) (DamageCauser :type Actor%20Object%20Reference))
  (bind _returnvalue (Transformation|GetActorLocation))
  (bind _sprite (Variables|Default|GetSprite))
  (if (not (Variables|Default|GetDie))
    (bind _output_get (Variables|Default|SetHP (Math|Float|Clamp(Float) (- (Variables|Default|GetHP) Damage) 0.0 (Variables|Default|GetHPLimit))))
    (bind _output_get_2 (Variables|Default|SetDie (== _output_get 0.0)))
    (Development|PrintString (Utilities|String|ToString(Float) (Variables|Default|GetHP)))
    (if _output_get_2
      (Audio|PlaySoundatLocation "/Game/Sounds/FREE_FPS_SFX_Pack/Enemy_Robot_Death-001.Enemy_Robot_Death-001" _returnvalue "0, 0, 0" 1.0 1.0 0.0 0 0 0 0)
      (Collision|SetCollisionEnabled (Variables|Collision|GetCapsuleComponent) "NoCollision")
      (Sprite|SetFlipbook _sprite "/Game/Textures/Doll/spr_Dem_Die/FB_DollDie.FB_DollDie")
      (Effects|SpawnEmitteratLocation 0 (Transformation|GetWorldLocation (Variables|Default|GetScene)))
      (Utilities|FlowControl|Delay (Class|PaperFlipbookComponent|GetFlipbookLength _sprite))
      (Actor|DestroyActor)
      (else
        (Audio|PlaySoundatLocation "/Game/Sounds/Damage_Grunt_Cue.Damage_Grunt_Cue" _returnvalue "0, 0, 0" 1.0 1.0 0.0 0 0 0 0)))))

(fn ConstructionScript)