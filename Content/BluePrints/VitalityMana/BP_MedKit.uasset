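; Health pickup actor that heals the player on touch and then destroys itself.
; On sphere overlap, it asks the player character through an interface message whether HP is maxed, and only acts if not.
; Healing goes through ApplyDamage with the DMT_Heal damage type, followed by a 2D sound.
; The construction script uses Type to pick the billboard sprite, plus scale, heal amount and sound pitch for the Low and Big variants.
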(event OnComponentBeginOverlap(Sphere)
  (params (OverlappedComponent :type Primitive%20Component%20Object%20Reference) (OtherActor :type Actor%20Object%20Reference) (OtherComp :type Primitive%20Component%20Object%20Reference) (OtherBodyIndex :type Integer) (bFromSweep :type Boolean) (SweepResult :type Hit%20Result%20Structure%20%28by%20ref%29))
  (bind _return (Class|BPIMedKit|GetCharacterHPMaxSignal(Message) (Game|GetPlayerCharacter 0)))
  (if (and (not _return) (== OtherActor (Game|GetPlayerCharacter 0)))
    (Game|Damage|ApplyDamage (Game|GetPlayerCharacter 0) (Variables|Default|GetAddHP) 0 self "/Game/BluePrints/VitalityMana/DMT_Heal.DMT_Heal_C")
    (Audio|PlaySound2D "/Game/Sounds/RetroGamePack/Retro_Game_Sounds_SFX_18.Retro_Game_Sounds_SFX_18" 0.4 (Variables|Default|GetPitchMultiplier) 0.03 0 0)
    (Actor|DestroyActor)))

(event EventBeginPlay)

(event Collision|EventActorBeginOverlap
  (params (OtherActor :type Actor%20Object%20Reference)))

(event EventTick
  (params (DeltaSeconds :type Float%20%28single-precision%29)))

(fn ConstructionScript
  (Utilities|FlowControl|Sequence
    (:then_0
      (switch Utilities|FlowControl|Switch|SwitchonEnum_MedKit (Variables|Default|GetType)
        (:NewEnumerator0
          (Variables|Default|SetSprite "/Game/Textures/Kits/health-green_32px.health-green_32px")
          (Transformation|SetWorldScale3D (Variables|Default|GetBillboard) "3.000000,1.000000,1.000000")
          (Variables|Default|SetAddHP 1e+01)
          (Variables|Default|SetPitchMultiplier 1.3))
        (:NewEnumerator1
          (Variables|Default|SetSprite "/Game/Textures/Kits/health-red_32px.health-red_32px")
          (Transformation|SetWorldScale3D (Variables|Default|GetBillboard) "5.000000,1.000000,1.000000")
          (Variables|Default|SetAddHP 25.0)
          (Variables|Default|SetPitchMultiplier 1.1))
        (:NewEnumerator2
          (Variables|Default|SetSprite "/Game/Textures/Kits/health-red_32px.health-red_32px"))))
    (:then_1
      (Rendering|Components|Sprite|SetSprite (Variables|Default|GetBillboard) (Variables|Default|GetSprite)))))

(fn GetCharacterHPMaxSignal
  (return false))