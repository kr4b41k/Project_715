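; DamagePlane is a hazard area actor that hurts the player while they stand inside its box.
; When the player character begins overlapping the box, it applies damage at once and starts a looping timer that repeats the hit at short intervals.
; Each hit applies a fixed amount with the DMT_Damage type, and leaving the box clears the timer.
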(event OnComponentBeginOverlap(Box)
  (params (OverlappedComponent :type Primitive%20Component%20Object%20Reference) (OtherActor :type Actor%20Object%20Reference) (OtherComp :type Primitive%20Component%20Object%20Reference) (OtherBodyIndex :type Integer) (bFromSweep :type Boolean) (SweepResult :type Hit%20Result%20Structure%20%28by%20ref%29))
  (if (== OtherActor (Game|GetPlayerCharacter 0))
    (bind _returnvalue (Utilities|Time|SetTimerbyEvent (delegate Custom|TakeDamage) 0.66 true))
    (Variables|Default|SetTimer _returnvalue)
    (Game|Damage|ApplyDamage (Game|GetPlayerCharacter 0) 5.0 0 self "/Game/BluePrints/VitalityMana/DMT_Damage.DMT_Damage_C")))

(event OnComponentEndOverlap(Box)
  (params (OverlappedComponent :type Primitive%20Component%20Object%20Reference) (OtherActor :type Actor%20Object%20Reference) (OtherComp :type Primitive%20Component%20Object%20Reference) (OtherBodyIndex :type Integer))
  (if (== OtherActor (Game|GetPlayerCharacter 0))
    (Utilities|Time|ClearandInvalidateTimerbyHandle (Variables|Default|GetTimer))))

(event Custom|TakeDamage
  (Game|Damage|ApplyDamage (Game|GetPlayerCharacter 0) 5.0 0 self "/Game/BluePrints/VitalityMana/DMT_Damage.DMT_Damage_C"))

(event EventBeginPlay)

(event Collision|EventActorBeginOverlap
  (params (OtherActor :type Actor%20Object%20Reference)))

(event EventTick
  (params (DeltaSeconds :type Float%20%28single-precision%29)))

(fn ConstructionScript)