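; BP_MedManaKit is a pickup that restores either health or mana to the player, selected by an HPMana setting.
; The construction script uses Type and HPMana to choose the billboard sprite, also setting scale and amount for all tiers except Free.
; On sphere overlap with the player character, it checks the max signal through message calls, then adds the amount and destroys itself only if not maxed.
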(event OnComponentBeginOverlap(Sphere)
  (params (OverlappedComponent :type Primitive%20Component%20Object%20Reference) (OtherActor :type Actor%20Object%20Reference) (OtherComp :type Primitive%20Component%20Object%20Reference) (OtherBodyIndex :type Integer) (bFromSweep :type Boolean) (SweepResult :type Hit%20Result%20Structure%20%28by%20ref%29))
  (bind _returnvalue (Game|GetPlayerCharacter 0))
  (bind _add (Variables|Default|GetAdd))
  (if (== OtherActor (Game|GetPlayerCharacter 0))
    (switch Utilities|FlowControl|Switch|SwitchonEnum_ManaMedKit (Variables|Default|GetHP_Mana)
      (:NewEnumerator0
        (bind _return (Class|BPIMedKit|GetCharacterHPMaxSignal(Message) (Game|GetPlayerCharacter 0)))
        (if (not _return)
          (Class|BPIHeal|AddHP(Message) _returnvalue _add)
          (Actor|DestroyActor :!label _label)))
      (:NewEnumerator1
        (bind _return_2 (Class|BPIMedKit|GetCharacterManaMaxSignal(Message) (Game|GetPlayerCharacter 0)))
        (if (not _return_2)
          (Class|BPIMana|AddMana(Message) _returnvalue _add)
          (goto _label))))))

(event EventBeginPlay)

(event Collision|EventActorBeginOverlap
  (params (OtherActor :type Actor%20Object%20Reference)))

(event EventTick
  (params (DeltaSeconds :type Float%20%28single-precision%29)))

(fn ConstructionScript
  (Utilities|FlowControl|Sequence
    (:then_0
      (switch Utilities|FlowControl|Switch|SwitchonEnum_MedKit (Variables|Default|GetType)
        (:NewEnumerator0
          (switch Utilities|FlowControl|Switch|SwitchonEnum_ManaMedKit (Variables|Default|GetHP_Mana)
            (:NewEnumerator0
              (Variables|Default|SetSprite "/Game/Textures/Kits/health-green_32px.health-green_32px"))
            (:NewEnumerator1
              (Variables|Default|SetSprite "/Game/Textures/Magic/ManaPotionLow.ManaPotionLow")))
          (Transformation|SetWorldScale3D (Variables|Default|GetBillboard) "3.000000,1.000000,1.000000")
          (Variables|Default|SetAdd 1e+01))
        (:NewEnumerator1
          (switch Utilities|FlowControl|Switch|SwitchonEnum_ManaMedKit (Variables|Default|GetHP_Mana)
            (:NewEnumerator0
              (Variables|Default|SetSprite "/Game/Textures/Kits/health-red_32px.health-red_32px"))
            (:NewEnumerator1
              (Variables|Default|SetSprite "/Game/Textures/Magic/ManaPotionMid.ManaPotionMid")))
          (Transformation|SetWorldScale3D (Variables|Default|GetBillboard) "5.000000,1.000000,1.000000")
          (Variables|Default|SetAdd 25.0))
        (:NewEnumerator2
          (switch Utilities|FlowControl|Switch|SwitchonEnum_ManaMedKit (Variables|Default|GetHP_Mana)
            (:NewEnumerator0
              (Variables|Default|SetSprite "/Game/Textures/Kits/health-red_32px.health-red_32px"))
            (:NewEnumerator1
              (Variables|Default|SetSprite "/Game/Textures/Magic/ManaPotionBig.ManaPotionBig"))))))
    (:then_1
      (Rendering|Components|Sprite|SetSprite (Variables|Default|GetBillboard) (Variables|Default|GetSprite)))))

(fn GetCharacterHPMaxSignal
  (return false))