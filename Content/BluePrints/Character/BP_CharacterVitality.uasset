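; BP_CharacterVitality is a character Blueprint that manages health and death.
; AnyDamage and AddHP clamp HP between zero and HPLimit, then push changes to an HP widget supplied through GetHPWidget.
; At zero HP, a DoOnce signals death to the widget, sets the Die flag and deactivates CharacterMovement.
; A query reports full HP, while the matching mana query always returns false.
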(event EventBeginPlay
  (|CallParentFunction)
  (Class|BPIWBHP|TakeHealSignal(Message) (Variables|Default|GetHPWidget) (Variables|Default|GetHP)))

(event Collision|EventActorBeginOverlap
  (params (OtherActor :type Actor%20Object%20Reference)))

(event EventTick
  (params (DeltaSeconds :type Float%20%28single-precision%29)))

(event Game|Damage|EventAnyDamage
  (params (Damage :type Float%20%28single-precision%29) (DamageType :type Damage%20Type%20Object%20Reference) (InstigatedBy :type Controller%20Object%20Reference) (DamageCauser :type Actor%20Object%20Reference))
  (if (not (Variables|Default|GetDie))
    (Variables|Default|SetDamage Damage)
    (Variables|Default|SetDamage%20Type DamageType)
    (Variables|Default|SetHP (Math|Float|Clamp(Float) (- (Variables|Default|GetHP) (Variables|Default|GetDamage)) 0.0 (Variables|Default|GetHP_Limit)))
    (if (!= (Variables|Default|GetHP) 0.0)
      (Class|BPIWBHP|TakeDamageSignal(Message) (Variables|Default|GetHPWidget) (Variables|Default|GetHP))
      (else
        (Utilities|FlowControl|DoOnce false
          (:Completed
            (Class|BPIWBHP|DIeSignal(Message) (Variables|Default|GetHPWidget))
            (Variables|Default|SetDie true)
            (Components|Activation|Deactivate (Variables|Character|GetCharacterMovement))))))))

(event EventGetHPWidget
  (params (HPWidget :type WB%20HP%20Object%20Reference))
  (bind _output_get (Variables|Default|SetHPWidget HPWidget))
  (Class|BPIWBHP|HPLimitSignal(Message) _output_get (Variables|Default|GetHP_Limit) (Variables|Default|GetHP)))

(event EventAddHP
  (params (HP :type Float%20%28double-precision%29))
  (Variables|Default|SetHP (Math|Float|Clamp(Float) (+ (Variables|Default|GetHP) HP) 0.0 (Variables|Default|GetHP_Limit)))
  (Class|BPIWBHP|TakeHealSignal(Message) (Variables|Default|GetHPWidget) (Variables|Default|GetHP)))

(fn ConstructionScript
  (|CallParentFunction))

(fn GetCharacterHPMaxSignal
  (return (== (Variables|Default|GetHP) (Variables|Default|GetHP_Limit))))

(fn GetCharacterManaMaxSignal
  (return false))