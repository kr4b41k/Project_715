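; BP_CharacterBase is a player character base with movement, look, jump and dash, all disabled when Die is set.
; Movement and jump inputs trigger camera animations, and BeginPlay creates the main HUD widget.
; A grounded dash locks forward movement to the camera vector, scales walk speed through a timeline, then runs a cooldown reported to DashWidget; releasing Shift ends it early.
; Shoot is a stub returning false.
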(event EventBeginPlay
  ;[1 0 0.4087] EventBeginPlay
  (Variables|Default|SetSpeed (Variables|/Script/Engine.CharacterMovementComponent|GetMaxWalkSpeed (Variables|Character|GetCharacterMovement)))
  (bind _returnvalue (UserInterface|CreateWidget "/Game/BluePrints/UI/WB_Main.WB_Main_C" (Game|GetPlayerController 0)))
  (bind _output_get (Variables|Default|SetMainWidget _returnvalue))
  (UserInterface|Viewport|AddtoViewport _output_get 0))

(event EventGetDashWidget
  (params (DashWidget :type WB%20Dash%20Object%20Reference))
  ;[0 1 1] Dash
  (Variables|Default|SetDash%20Widget DashWidget))

(event Input|AxisEvents|InputAxisMoveForwardInput
  (params (AxisValue :type Float%20%28single-precision%29))
  ;[0 1 0.4161] MoveMent
  (if (not (Variables|Default|GetDie))
    (if (Variables|Default|GetCameraDashLock)
      (Pawn|Input|AddMovementInput (Variables|Default|GetCameraDashVector) AxisValue false)
      (else
        (Pawn|Input|AddMovementInput (Transformation|GetActorForwardVector) AxisValue false)))))

(event Input|AxisEvents|InputAxisMoveRightInput
  (params (AxisValue :type Float%20%28single-precision%29))
  ;[0 1 0.4161] MoveMent
  (if (not (Variables|Default|GetDie))
    (Pawn|Input|AddMovementInput (Transformation|GetActorRightVector) AxisValue false)))

(event Input|AxisEvents|InputAxisCameraUpInput
  (params (AxisValue :type Float%20%28single-precision%29))
  ;[0 1 0.4161] MoveMent
  (if (not (Variables|Default|GetDie))
    (Pawn|Input|AddControllerPitchInput (* AxisValue (Variables|Default|GetSensevity)))))

(event Input|AxisEvents|InputAxisCameraRightInput
  (params (AxisValue :type Float%20%28single-precision%29))
  ;[0 1 0.4161] MoveMent
  (if (not (Variables|Default|GetDie))
    (Pawn|Input|AddControllerYawInput (* AxisValue (Variables|Default|GetSensevity)))))

(event Input|KeyboardEvents|SpaceBar
  (params (Key :type Key%20Structure :default "None"))
  ;[0 1 0.4161] MoveMent
  (:Pressed
    (if (not (Variables|Default|GetDie))
      (Character|Jump)
      (if (not (AI|Components|NavMovement|IsFalling (Variables|Character|GetCharacterMovement)))
        (CameraAnimation|PlayCameraAnimation (Subsystems|GetGameplayCamerasSubsystem) (Game|GetPlayerController 0) "/Game/CameraAnimations/MoveMent/Jump.Jump" :!class /Script/GameplayCameras.GameplayCamerasSubsystem)
        (Audio|PlaySound2D "/Game/Sounds/FPS_Pack/SND_Jump_Cue.SND_Jump_Cue" 1.0 1.0 0.0 0 0)))))

(event Input|KeyboardEvents|LeftShift
  (params (Key :type Key%20Structure :default "None"))
  (bind _charactermovement (Variables|Character|GetCharacterMovement))
  (bind _die (Variables|Default|GetDie))
  (bind _returnvalue (not _die))
  ;[0 1 1] Dash
  (:Pressed
    (if _returnvalue
      (if (and (Variables|Default|GetDashAvaible) (not (AI|Components|NavMovement|IsFalling (Variables|Character|GetCharacterMovement))))
        (Utilities|FlowControl|Sequence
          (:then_0
            (Variables|Default|SetDashAvaible false)
            (Variables|Default|SetCameraDashVector (Math|Vector|GetForwardVector (Variables|Default|GetCamera)))
            (Variables|Default|SetCameraDashLock true)
            (bind _alpha (Timeline|Dash PlayFromStart)
              (:Update
                (Variables|/Script/Engine.CharacterMovementComponent|SetMaxWalkSpeed _charactermovement (* _alpha (Variables|Default|GetSpeed) (Variables|Default|GetDashForce))))
              (:Finished
                (Variables|Default|SetCameraDashLock false :!label _label)
                (Variables|/Script/Engine.CharacterMovementComponent|SetMaxWalkSpeed _charactermovement (Variables|Default|GetSpeed))
                (Utilities|FlowControl|Sequence
                  (:then_0
                    (Utilities|FlowControl|Delay (Variables|Default|GetDashCoolDown))
                    (Variables|Default|SetDashAvaible true)
                    (Audio|PlaySound2D "/Game/Sounds/FPS_Pack/SND_Jump_Cue.SND_Jump_Cue" 2.5 0.8 0.02 0 0)
                    (Class|BPIWBDash|DashAvaibleSignal(Message) (Variables|Default|GetDash%20Widget))
                    (Variables|Default|SetDashRegen false))
                  (:then_1
                    (if (not (Variables|Default|GetDashRegen))
                      (Class|BPIWBDash|DashRegenSignal(Message) (Variables|Default|GetDash%20Widget) (Variables|Default|GetDashCoolDown))
                      (Variables|Default|SetDashRegen true)))))))
          (:then_1
            (CameraAnimation|PlayCameraAnimation (Subsystems|GetGameplayCamerasSubsystem) (Game|GetPlayerController 0) "/Game/CameraAnimations/MoveMent/Dash.Dash" :!class /Script/GameplayCameras.GameplayCamerasSubsystem)
            (Audio|PlaySound2D "/Game/Sounds/FREE_FPS_SFX_Pack/Player_Jump.Player_Jump" 1.0 1.0 0.0 0 0)
            (Class|BPIWBDash|DashSignal(Message) (Variables|Default|GetDash%20Widget))))
        (else
          (Class|BPIWBDash|DashNotAvaibleSignal(Message) (Variables|Default|GetDash%20Widget))))))
  (:Released
    (if _returnvalue
      (if (not (Variables|Default|GetDashAvaible))
        (Utilities|FlowControl|Sequence
          (:then_0
            (Timeline|Dash Stop))
          (:then_1
            (goto _label)))))))

(event Input|KeyboardEvents|W
  (params (Key :type Key%20Structure :default "None"))
  ;[1 0.2658 0] StrafeShake
  (:Pressed
    (if (not (Variables|Default|GetDie))
      (CameraAnimation|PlayCameraAnimation (Subsystems|GetGameplayCamerasSubsystem) (Game|GetPlayerController 0) "/Game/CameraAnimations/MoveMent/ForwardStrafe.ForwardStrafe" :!class /Script/GameplayCameras.GameplayCamerasSubsystem))))

(event Input|KeyboardEvents|A
  (params (Key :type Key%20Structure :default "None"))
  ;[1 0.2658 0] StrafeShake
  (:Pressed
    (if (not (Variables|Default|GetDie))
      (CameraAnimation|PlayCameraAnimation (Class|CameraAnimationCameraModifier|GetCameraAnimationCameraModifier) "/Game/CameraAnimations/MoveMent/RightStrafe.RightStrafe" (Utilities|Struct|MakeCameraAnimationParams 1.0 -1.0 "Linear" 0.0 "Linear" 0.0 false 0 false 0.0 "CameraLocal" "0.000000,0.000000,0.000000") :!class /Script/GameplayCameras.CameraAnimationCameraModifier))))

(event Input|KeyboardEvents|D
  (params (Key :type Key%20Structure :default "None"))
  ;[1 0.2658 0] StrafeShake
  (:Pressed
    (if (not (Variables|Default|GetDie))
      (CameraAnimation|PlayCameraAnimation :self (Class|CameraAnimationCameraModifier|GetCameraAnimationCameraModifier) :Sequence "/Game/CameraAnimations/MoveMent/RightStrafe.RightStrafe" :!class /Script/GameplayCameras.CameraAnimationCameraModifier))))

(fn ConstructionScript)

(fn Shoot
  (return false))