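; Character Blueprint that handles the player's equipped weapon, starting with a pistol-style BP_Gun and switching to machine gun, shotgun or Gutlin.
; Switch inputs check ammo stored in the Core, then destroy the old actor, spawn and attach the new one, and record the selection.
; Fire input and the ammo widget reach the weapon through signal messages.
; Separate signal events store and play camera animations on the player camera manager.
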(event Custom|SpawnWeapon
  (bind _self self)
  (bind _returnvalue (Game|SpawnActorfromClass (Variables|Default|GetCurrentWeapon) (Transformation|GetActorTransform) "AlwaysSpawn" "MultiplyWithRoot" _self 0 _self))
  (Variables|Default|SetEquipedWeapon _returnvalue)
  (Transformation|AttachComponentToComponent _returnvalue (Variables|Default|GetScene) "None" "SnapToTarget" "SnapToTarget" "SnapToTarget" false)
  (Class|BPIWeaponUse|SwitchSignal(Message) (Variables|Default|GetEquipedWeapon) (Variables|Default|GetAmmo%20Widget)))

(event Custom|DestroyWeapon
  (Actor|DestroyActor (Variables|Default|GetEquipedWeapon)))

(event EventGetAmmoWidget
  (params (AmmoWidget :type WB%20Ammo%20Object%20Reference))
  (Variables|Default|SetAmmo%20Widget AmmoWidget))

(event EventBeginPlay
  (bind _self self)
  (|CallParentFunction)
  (Variables|Default|SetCurrentWeapon "/Game/BluePrints/Weapon/Guns/BP_Gun.BP_Gun_C")
  (bind _returnvalue (Game|SpawnActorfromClass (Variables|Default|GetCurrentWeapon) (Transformation|GetActorTransform) "AlwaysSpawn" "MultiplyWithRoot" _self 0 _self))
  (Variables|Default|SetEquipedWeapon _returnvalue)
  (Transformation|AttachComponentToComponent _returnvalue (Variables|Default|GetScene) "None" "SnapToTarget" "SnapToTarget" "SnapToTarget" false)
  (Class|BPIWeaponUse|SwitchSignal(Message) (Variables|Default|GetEquipedWeapon) (Variables|Default|GetAmmo%20Widget)))

(event EventCameraAnimSignalPlayer
  (params (CameraAnimation :type Camera%20Animation%20Sequence%20Object%20Reference))
  (Variables|Default|SetCurrentCameraAnimation CameraAnimation))

(event EventCameraAnimPlaySignalPlayer
  (CameraAnimation|PlayCameraAnimation :self (CameraAnimation|ConvCameraAnimationCameraModifier (Game|GetPlayerCameraManager 0)) :Sequence (Variables|Default|GetCurrentCameraAnimation) :!class /Script/GameplayCameras.CameraAnimationCameraModifier))

(event Input|ActionEvents|InputActionSwitchOnGun
  (params (Key :type Key%20Structure :default "None"))
  (:Pressed
    (if (not (Variables|Default|GetDie))
      (Variables|Default|SetEnumWeapon "NewEnumerator0")
      (if (!= (Variables|/Game/BluePrints/GI_Core.GI_Core_C|GetCurrentGunAmmo (CallFunction|GetCore)) 0)
        (CallFunction|DestroyWeapon)
        (Variables|Default|SetCurrentWeapon "/Game/BluePrints/Weapon/Guns/BP_Gun.BP_Gun_C")
        (CallFunction|SpawnWeapon)
        (Variables|/Game/BluePrints/GI_Core.GI_Core_C|SetCurrentWeapon (CallFunction|GetCore) (Variables|Default|GetEnumWeapon))
        (Class|BPIWeaponUse|SwitchSignal(Message) (Variables|Default|GetEquipedWeapon) (Variables|Default|GetAmmo%20Widget))))))

(event Input|ActionEvents|InputActionSwitchOnMachineGun
  (params (Key :type Key%20Structure :default "None"))
  (:Pressed
    (if (not (Variables|Default|GetDie))
      (Variables|Default|SetEnumWeapon "NewEnumerator1")
      (if (!= (Variables|/Game/BluePrints/GI_Core.GI_Core_C|GetCurrentMachineGunAmmo (CallFunction|GetCore)) 0)
        (CallFunction|DestroyWeapon)
        (Variables|Default|SetCurrentWeapon "/Game/BluePrints/Weapon/Guns/BP_MachineGun.BP_MachineGun_C")
        (CallFunction|SpawnWeapon)
        (Variables|/Game/BluePrints/GI_Core.GI_Core_C|SetCurrentWeapon (CallFunction|GetCore) (Variables|Default|GetEnumWeapon))
        (Class|BPIWeaponUse|SwitchSignal(Message) (Variables|Default|GetEquipedWeapon) (Variables|Default|GetAmmo%20Widget))))))

(event Input|ActionEvents|InputActionSwitchOnShotGun
  (params (Key :type Key%20Structure :default "None"))
  (:Pressed
    (if (not (Variables|Default|GetDie))
      (Variables|Default|SetEnumWeapon "NewEnumerator2")
      (if (!= (Variables|/Game/BluePrints/GI_Core.GI_Core_C|GetCurrentShotGunAmmo (CallFunction|GetCore)) 0)
        (CallFunction|DestroyWeapon)
        (Variables|Default|SetCurrentWeapon "/Game/BluePrints/Weapon/Guns/BP_ShotGun.BP_ShotGun_C")
        (CallFunction|SpawnWeapon)
        (Variables|/Game/BluePrints/GI_Core.GI_Core_C|SetCurrentWeapon (CallFunction|GetCore) (Variables|Default|GetEnumWeapon))
        (Class|BPIWeaponUse|SwitchSignal(Message) (Variables|Default|GetEquipedWeapon) (Variables|Default|GetAmmo%20Widget))))))

(event Input|ActionEvents|InputActionSwitchOnGutlin
  (params (Key :type Key%20Structure :default "None"))
  (:Pressed
    (if (not (Variables|Default|GetDie))
      (Variables|Default|SetEnumWeapon "NewEnumerator3")
      (if (!= (Variables|/Game/BluePrints/GI_Core.GI_Core_C|GetCurrentGutlinAmmo (CallFunction|GetCore)) 0)
        (CallFunction|DestroyWeapon)
        (Variables|Default|SetCurrentWeapon "/Game/BluePrints/Weapon/Guns/BP_Gutlin.BP_Gutlin_C")
        (CallFunction|SpawnWeapon)
        (Variables|/Game/BluePrints/GI_Core.GI_Core_C|SetCurrentWeapon (CallFunction|GetCore) (Variables|Default|GetEnumWeapon))
        (Class|BPIWeaponUse|SwitchSignal(Message) (Variables|Default|GetEquipedWeapon) (Variables|Default|GetAmmo%20Widget))))))

(event Input|ActionEvents|InputActionSwitchOnBazooka
  (params (Key :type Key%20Structure :default "None")))

(event Input|MouseEvents|LeftMouseButton
  (params (Key :type Key%20Structure :default "None"))
  (bind _equipedweapon (Variables|Default|GetEquipedWeapon))
  (bind _equipedweapon_2 (Variables|Default|GetEquipedWeapon))
  (bind _die (Variables|Default|GetDie))
  (bind _returnvalue (not _die))
  (:Pressed
    (if _returnvalue
      (Utilities|IsValid _equipedweapon
        (:Is%20Valid
          (Class|BPIWeaponUse|ShootSignal(Message) _equipedweapon)))))
  (:Released
    (if _returnvalue
      (Utilities|IsValid _equipedweapon_2
        (:Is%20Valid
          (Class|BPIWeaponUse|StopShootSignal(Message) _equipedweapon_2))))))

(fn ConstructionScript
  (|CallParentFunction))

(fn GetAmmoFull
  (return false))